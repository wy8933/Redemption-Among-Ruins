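; Dialogue component for the NPC Bob, covering the outbreak's backstory and a later helicopter fuel-or-defend conversation.
; Overrides Dialogue, calls the parent, then branches on DialogueTreeIndex through chained AddDialogue calls gated by DialogueState and OptionIndex.
; Finishing the backstory or skipping it advances the tree to the helicopter stage; endings clear progress and close the conversation.
; The helicopter choice switches on constant 0, so only the fuel reply runs.
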(fn Dialogue
  (|CallParentFunction)
  (switch int (Variables|Default|GetDialogueTreeIndex)
    (:0
      (bind (_dialoguestate _optionindex) (CallFunction|AddDialogue "Bob(holding the wound, in pain but urgent)" "Careful with that trigger! We've got bigger problems than stray bullets. This chaos... it's not just happening. There's a reason behind it." (Utilities|Array|MakeArray "\"I'm really sorry about that. But what do you mean? What's causing all this?" "I didn't mean to... But yes, what's going on here? It's like the whole town's gone mad." "We're all on edge. Let's focus on getting out of here alive. 
(Skip background story)"))) ; 0
      (switch Utilities|FlowControl|Switch|SwitchonEnum_DialogueState _dialoguestate
        (:NewEnumerator0
          (switch int _optionindex
            (:0
              (bind (_dialoguestate_2 _optionindex_2) (CallFunction|AddDialogue "Bob" "This outbreak, it's not a natural disaster. It's man-made, a catastrophe born from ambition and curiosity gone wrong. You've heard of Dr. Maddox, right? Moved here a while back, took up a position at the Memorial Hospital. She was onto something, something big and dangerous." (Utilities|Array|MakeArray "Dr. Maddox? The virologist? How is she involved in this?" "I've heard rumors, but... how could research turn into... this?") :!label _label))
              (switch Utilities|FlowControl|Switch|SwitchonEnum_DialogueState _dialoguestate_2
                (:NewEnumerator0
                  (switch int _optionindex_2
                    (:0
                      _)
                    (:1
                      _))
                  (bind (_dialoguestate_3 _optionindex_3) (CallFunction|AddDialogue "Bob" "Maddox found a virus, ancient and dormant, buried right here in our backyard. She thought it could revolutionize medicine. But instead of healing, it brought ruin. It escaped the lab, and now, here we are, fighting for our lives in what's left of our town." (Utilities|Array|MakeArray "This is insane... So, what now? How do we survive this?")))
                  (switch Utilities|FlowControl|Switch|SwitchonEnum_DialogueState _dialoguestate_3
                    (:NewEnumerator0
                      (switch int _optionindex_3
                        (:0
                          (CallFunction|AddDialogue "Bob" "Survival's in our blood; we're descendants of pioneers. But first, we need to get you patched up and out of this plaza. There's a helicopter coming. We'll head to the hospital, find supplies, and maybe, just maybe, find a clue to stopping this nightmare." (Utilities|Array|MakeArray "Continue"))
                          (switch Utilities|FlowControl|Switch|SwitchonEnum_DialogueState "NewEnumerator0"
                            (:NewEnumerator0
                              (CallFunction|SetDialogueTreeIndex 1)
                              (CallFunction|ClearDialogueProgress)
                              (CallFunction|CloseConversation))))))))))
            (:1
              (goto _label))
            (:2
              (bind _dialoguestate_4 (CallFunction|AddDialogue "Bob" "Alright, no time to dwell on it. We need to get to a safer place, and you need to cover me." (Utilities|Array|MakeArray "Let's go")))
              (switch Utilities|FlowControl|Switch|SwitchonEnum_DialogueState _dialoguestate_4
                (:NewEnumerator0
                  (CallFunction|SetDialogueTreeIndex 1)
                  (CallFunction|ClearDialogueProgress)
                  (CallFunction|CloseConversation))))))))
    (:1
      (bind _dialoguestate_5 (CallFunction|AddDialogue "Bob" "This isn't your standard chopper; those symbols... they mean it's off-limits. But it might be our only shot at getting out. We've got two options: find fuel to get it airborne or stay and defend it from those things. What do you think?" (Utilities|Array|MakeArray "I'll go for the fuel. We can't let this chance slip. Keep the helicopter safe until I get back." "We should defend the helicopter first. You find any fuel cans around; I'll keep the infected away.")))
      (switch Utilities|FlowControl|Switch|SwitchonEnum_DialogueState _dialoguestate_5
        (:NewEnumerator0
          (switch int 0
            (:0
              (bind _dialoguestate_6 (CallFunction|AddDialogue "Bob" "Got it. I'll hold the fort here. Be quick, and watch your back. The noise from this bird's going to attract a lot of unwanted attention."))
              (switch Utilities|FlowControl|Switch|SwitchonEnum_DialogueState _dialoguestate_6
                (:NewEnumerator0
                  _)))
            (:1
              (bind _dialoguestate_7 (CallFunction|AddDialogue "Bob" "Alright, if you're sure. I saw some fuel cans back at the plaza. I'll be as fast as I can. Just keep them off me and this helicopter."))
              (switch Utilities|FlowControl|Switch|SwitchonEnum_DialogueState _dialoguestate_7
                (:NewEnumerator0
                  _))))
          (CallFunction|ClearDialogueProgress)
          (CallFunction|CloseConversation))))))