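; Dialogue component for the intro conversation, in which a wounded Bob explains the virus outbreak behind the town's chaos.
; Dialogue branches on DialogueTreeIndex, with chained AddDialogue calls supplying speaker, line and player options.
; The first two replies share the backstory path, which sets the index to 1 and closes; the skip reply only adds a short line.
; Index 1 plays a Black Smith line, then clears progress and closes.
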(event EventBeginPlay
  (|CallParentFunction) ; This node is disabled and will not be called.\nDrag off pins to build functionality.
)

(event EventTick
  (params (DeltaSeconds :type Float%20%28single-precision%29))
  (|CallParentFunction DeltaSeconds) ; This node is disabled and will not be called.\nDrag off pins to build functionality.
)

(fn Dialogue
  (|CallParentFunction)
  (switch int (Variables|Default|GetDialogueTreeIndex)
    (:0
      (|IntroductionBackgroundStory))
    (:1
      (bind _dialoguestate (CallFunction|AddDialogue "Black Smith" "Great deal with you last time" (Utilities|Array|MakeArray "Continue")))
      (switch Utilities|FlowControl|Switch|SwitchonEnum_DialogueState _dialoguestate
        (:NewEnumerator0
          (CallFunction|ClearDialogueProgress)
          (CallFunction|CloseConversation))))))