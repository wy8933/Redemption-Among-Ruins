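; Blacksmith dialogue component that overrides the parent Dialogue function to script a branching weapon-sale conversation; the purchase is dialogue only.
; Nested AddDialogue calls branch on the chosen option and continue on Pass Through.
; DialogueTreeIndex selects the tree, and completing the deal switches it to a returning-customer greeting.
; Deferring rewinds two progress steps to resume the offer later, while refusing clears progress.
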(fn Dialogue
  (|CallParentFunction)
  (switch int (Variables|Default|GetDialogueTreeIndex)
    (:0
      (bind (_dialoguestate _optionindex) (CallFunction|AddDialogue "Black Smith" "Hi, wanna get some weapon?" (Utilities|Array|MakeArray "Oh yes" "No you"))) ; 0
      (switch Utilities|FlowControl|Switch|SwitchonEnum_DialogueState _dialoguestate
        (:NewEnumerator0
          (switch int _optionindex
            (:0
              (bind (_dialoguestate_2 _optionindex_2) (CallFunction|AddDialogue "Black Smith" "$10000000 for a ak-47" (Utilities|Array|MakeArray "I will pay in cash" "I will come back later"))) ; 1
              (switch Utilities|FlowControl|Switch|SwitchonEnum_DialogueState _dialoguestate_2
                (:NewEnumerator0
                  (switch int _optionindex_2
                    (:0
                      (bind _dialoguestate_3 (CallFunction|AddDialogue "Black Smith" "Thank you for the deal" (Utilities|Array|MakeArray "Bye")))
                      (switch Utilities|FlowControl|Switch|SwitchonEnum_DialogueState _dialoguestate_3
                        (:NewEnumerator0
                          (CallFunction|SetDialogueTreeIndex 1)
                          (CallFunction|CloseConversation))))
                    (:1
                      (bind _dialoguestate_4 (CallFunction|AddDialogue "Black Smith" "Ok see you later" (Utilities|Array|MakeArray "Continue")))
                      (switch Utilities|FlowControl|Switch|SwitchonEnum_DialogueState _dialoguestate_4
                        (:NewEnumerator0
                          (CallFunction|RemoveDialogueProgress 2) ; Go back  a few step in the conversation, that you will be at the same state when you come back again
                          (CallFunction|CloseConversation))))))))
            (:1
              (bind _dialoguestate_5 (CallFunction|AddDialogue "Black Smith" "get out of here" (Utilities|Array|MakeArray "Chill out"))) ; 1
              (switch Utilities|FlowControl|Switch|SwitchonEnum_DialogueState _dialoguestate_5
                (:NewEnumerator0
                  ;[1 1 1] End converstation
                  (CallFunction|ClearDialogueProgress)
                  (CallFunction|CloseConversation))))))))
    (:1
      (bind _dialoguestate_6 (CallFunction|AddDialogue "Black Smith" "Great deal with you last time" (Utilities|Array|MakeArray "Continue")))
      (switch Utilities|FlowControl|Switch|SwitchonEnum_DialogueState _dialoguestate_6
        (:NewEnumerator0
          (CallFunction|ClearDialogueProgress)
          (CallFunction|CloseConversation))))))