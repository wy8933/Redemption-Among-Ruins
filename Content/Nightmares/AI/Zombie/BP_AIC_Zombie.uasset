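; AI controller for the zombie enemy that runs BT_Zombie on the server at BeginPlay.
; The AIPerception component stores a sensed player-controlled character as the blackboard Target and clears it when sensing is lost.
; A separate Hearing perception component writes the stimulus location and heard state to the blackboard for player characters.
; A third perception component, AIPerception1, only prints a debug string on updates.
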(event OnTargetPerceptionUpdated(Hearing)
  (params (Actor :type Actor%20Object%20Reference) (Stimulus :type AI%20Stimulus%20Structure))
  (bind (_age _expirationage _strength _stimuluslocation _receiverlocation _tag _bsuccessfullysensed) (Utilities|Struct|BreakAIStimulus Stimulus))
  (bind _ascharacter (Utilities|Casting|CastToCharacter Actor))
  (if (Pawn|IsPlayerControlled _ascharacter)
    (Variables|Default|SetHearingLocation _stimuluslocation)
    (Variables|Default|SetHeard _bsuccessfullysensed)
    (AI|Components|Blackboard|SetValueasVector (AI|GetBlackboard 0) (Utilities|Name|MakeLiteralName "HearingLocation") (Variables|Default|GetHearingLocation))
    (AI|Components|Blackboard|SetValueasBool (AI|GetBlackboard 0) (Utilities|Name|MakeLiteralName "Hearing") (Variables|Default|GetHeard))))

(event OnTargetPerceptionUpdated(AIPerception)
  (params (Actor :type Actor%20Object%20Reference) (Stimulus :type AI%20Stimulus%20Structure))
  (bind _ascharacter (Utilities|Casting|CastToCharacter Actor))
  (if (Pawn|IsPlayerControlled _ascharacter)
    (if (.bSuccessfullySensed (Utilities|Struct|BreakAIStimulus Stimulus))
      (AI|Components|Blackboard|SetValueasObject (AI|GetBlackboard 0) (Utilities|Name|MakeLiteralName "Target") Actor)
      (else
        (AI|Components|Blackboard|SetValueasObject (AI|GetBlackboard 0) (Utilities|Name|MakeLiteralName "Target") 0)))))

(event OnTargetPerceptionUpdated(AIPerception1)
  (params (Actor :type Actor%20Object%20Reference) (Stimulus :type AI%20Stimulus%20Structure))
  (Development|PrintString "Hello"))

(fn ConstructionScript)

(fn ReceiveBeginPlay
  (if (Networking|IsServer)
    (AI|RunBehaviorTree "/Game/Nightmares/AI/Zombie/BT_Zombie.BT_Zombie")))