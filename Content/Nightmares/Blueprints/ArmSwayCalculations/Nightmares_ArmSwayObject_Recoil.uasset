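; Arm sway calculation object for Nightmares that outputs a smoothed recoil location and rotation offset.
; Each Output call interpolates the final offset toward the current recoil values, while those recoil values interpolate back toward zero.
; This two-stage chase eases a recoil kick in and out; nothing in this graph sets the recoil values themselves.
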(fn Output
  (params (Delta :type Float%20%28double-precision%29))
  (bind _returnvalue (Math|Float|MakeLiteralFloat 1e+01))
  (bind _returnvalue_2 (Math|Float|MakeLiteralFloat 1e+01))
  (Variables|Default|SetFinalLocation (Math|Interpolation|VInterpTo (Variables|Default|GetFinalLocation) (Variables|Default|GetRecoilLocation) Delta _returnvalue))
  (Variables|Default|SetFinalRotation (Math|Interpolation|RInterpTo (Variables|Default|GetFinalRotation) (Variables|Default|GetRecoilRotation) Delta _returnvalue))
  (Variables|Default|SetRecoilLocation (Math|Interpolation|VInterpTo (Variables|Default|GetRecoilLocation) "0, 0, 0" Delta _returnvalue_2))
  (Variables|Default|SetRecoilRotation (Math|Interpolation|RInterpTo (Variables|Default|GetRecoilRotation) "0, 0, 0" Delta _returnvalue_2))
  (return (Variables|Default|GetFinalLocation) (Variables|Default|GetFinalRotation)))