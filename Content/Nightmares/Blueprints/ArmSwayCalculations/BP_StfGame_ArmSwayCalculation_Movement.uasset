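; Arm sway calculation that turns the character's movement into location and rotation offsets, producing a bob while moving.
; Smoothed horizontal speed, targeting zero during any vertical motion, sets both how fast a vector curve is sampled and how strongly it scales the location offset.
; The rotation offset interpolates toward a clamped pitch from vertical velocity and a yaw from the scaled curve's Y component.
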(fn Output
  (params (Delta :type Float%20%28double-precision%29))
  (bind _character (Variables|Default|GetCharacter))
  (bind _returnvalue (Transformation|GetVelocity _character))
  (bind (_x _y) (Math|Vector|BreakVector _returnvalue))
  (Variables|Default|SetCharacterSpeed (Math|Interpolation|FInterpTo (Variables|Default|GetCharacterSpeed) (select (> (Math|Vector|VectorLength (Math|Vector|MakeVector 0.0 0.0 (.Z (Math|Vector|BreakVector (Transformation|GetVelocity (Variables|Default|GetCharacter)))))) 0.0) 0.0 (Math|Vector|VectorLength (Math|Vector|MakeVector _x _y 0.0))) Delta 5.0))
  (Variables|Default|SetTime (+ (Variables|Default|GetTime) (* Delta (Math|Float|MapRangeClamped (Variables|Default|GetCharacterSpeed) 3e+02 6e+02 2.25 3.5))))
  (Variables|Default|SetNewVar (Math|Interpolation|RInterpTo (Variables|Default|GetNewVar) (Math|Rotator|MakeRotator 0.0 (Math|Float|ClampAngle (/ (.Z (Math|Vector|BreakVector (Transformation|GetVelocity (Variables|Default|GetCharacter)))) -35.0) -45.0 45.0) (* (.Y (Math|Vector|BreakVector (* (Math|Vector|MakeVector (.X (Math|Vector|BreakVector (Math|Curves|GetVectorValue (LocalVariables|GetCurve) (Variables|Default|GetTime)))) (* (.Y (Math|Vector|BreakVector (Math|Curves|GetVectorValue (LocalVariables|GetCurve) (Variables|Default|GetTime)))) 0.5) (* (.Z (Math|Vector|BreakVector (Math|Curves|GetVectorValue (LocalVariables|GetCurve) (Variables|Default|GetTime)))) 0.5)) (Math|Float|MapRangeClamped (Variables|Default|GetCharacterSpeed) 1e+02 6e+02 0.0 2.0)))) -1.5)) Delta 25.0))
  (return (* (Math|Vector|MakeVector (.X (Math|Vector|BreakVector (Math|Curves|GetVectorValue (LocalVariables|GetCurve) (Variables|Default|GetTime)))) (* (.Y (Math|Vector|BreakVector (Math|Curves|GetVectorValue (LocalVariables|GetCurve) (Variables|Default|GetTime)))) 0.5) (* (.Z (Math|Vector|BreakVector (Math|Curves|GetVectorValue (LocalVariables|GetCurve) (Variables|Default|GetTime)))) 0.5)) (Math|Float|MapRangeClamped (Variables|Default|GetCharacterSpeed) 1e+02 6e+02 0.0 2.0)) (Variables|Default|GetNewVar)))