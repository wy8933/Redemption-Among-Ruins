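; Arm sway calculation object that produces a lagging rotation offset from the character's look movement.
; Each Output call takes the change in control rotation since the previous call, inverts it and clamps pitch and yaw to a small range, with roll zeroed.
; An interpolated rotation eases toward that target and is returned as the rotation offset, with a zero location offset.
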(fn Output
  (params (Delta :type Float%20%28double-precision%29))
  (bind _character (Variables|Default|GetCharacter))
  (bind _returnvalue (Pawn|GetControlRotation _character :!class /Script/Engine.Pawn))
  (LocalVariables|SetOffset (Math|Rotator|Delta(Rotator) _returnvalue (Variables|Default|GetControlRotation)))
  (Variables|Default|SetControlRotation _returnvalue)
  (Variables|Default|SetFinalRotation (Math|Interpolation|RInterpTo (Variables|Default|GetFinalRotation) (Math|Rotator|MakeRotator 0.0 (Math|Float|Clamp(Float) (.Pitch (Math|Rotator|BreakRotator (* (LocalVariables|GetOffset) -1.0))) -5.0 5.0) (Math|Float|Clamp(Float) (.Yaw (Math|Rotator|BreakRotator (* (LocalVariables|GetOffset) -1.0))) -5.0 5.0)) Delta 7.0))
  (return "0, 0, 0" (Variables|Default|GetFinalRotation)))