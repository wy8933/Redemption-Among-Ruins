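; Player controller for Nightmares that handles on-foot input, HUD switching, death and respawn requests.
; Enhanced Input drives camera-relative movement, slowed when aiming and fastest when sprinting forward, and look sensitivity scaled by FOV.
; Keys open inventory and pause menus, while events handle character selection, suicide, respawn through the GameMode, lobby travel and Sinister Hunt messages.
; Die sets the dead HUD and flag, but the automatic respawn in Tick is disconnected.
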(event Custom|ServerSpawn
  (CallFunction|Spawn))

(event Custom|ServerSelectCharacter
  (params (CharacterClass :type Pawn%20Class%20Reference))
  (Variables|Default|SetCharacterClass CharacterClass))

(event Custom|ServerLobby
  (Development|ExecuteConsoleCommand "servertravel /Game/Nightmares/Levels/Lobby" 0))

(event Custom|ClientSendMessage
  (params (Name :type String) (Count :type String))
  (bind _foundwidgets (Widget|GetAllWidgetsOfClass "/Game/Nightmares/UserWidgets/Game/WBP_SinisterHunt_School.WBP_SinisterHunt_School_C" false))
  (Default|AddMessage (Utilities|Array|Get(acopy) _foundwidgets) Name Count))

(event Custom|ServerSuiside
  (bind _asnightmares_character (Utilities|Casting|CastToNightmares_Character (Pawn|GetControlledPawn)))
  (Default|Die _asnightmares_character (Variables|GetPlayerState)))

(event Input|EnhancedActionEvents|EnhancedInputActionIA_OniKami_Move
  (params (ActionValue :type Vector%202D%20Structure) (ElapsedSeconds :type Float%20%28double-precision%29) (TriggeredSeconds :type Float%20%28double-precision%29) (InputAction :type Input%20Action%20Object%20Reference :default "/Game/Nightmares/Inputs/IA_OniKami_Move.IA_OniKami_Move"))
  (bind _returnvalue (Pawn|GetControlledPawn))
  (bind _returnvalue_2 (Pawn|GetControlRotation :!class /Script/Engine.Controller))
  (bind _returnvalue_3 (Math|Vector2D|Normalize2D ActionValue))
  (bind _yaw (Math|Rotator|BreakRotator _returnvalue_2))
  (bind _returnvalue_4 (Math|Rotator|MakeRotator 0.0 0.0 _yaw))
  (bind _asnightmares_character (Utilities|Casting|CastToNightmares_Character _returnvalue))
  (Pawn|Input|AddMovementInput _returnvalue (Math|Vector|GetForwardVector _returnvalue_4) (.X (Math|Vector2D|BreakVector2D (* _returnvalue_3 (select (Variables|/Game/Nightmares/Blueprints/Characters/Nightmares_Character.Nightmares_Character_C|GetIsADS _asnightmares_character) 0.25 (select (and (> (.X (Math|Vector2D|BreakVector2D _returnvalue_3)) 0.0) (Variables|Default|GetIsSprinting)) 1.0 0.5))))) false)
  (Pawn|Input|AddMovementInput _returnvalue (Math|Vector|GetRightVector _returnvalue_4) (.Y (Math|Vector2D|BreakVector2D (* _returnvalue_3 (select (Variables|/Game/Nightmares/Blueprints/Characters/Nightmares_Character.Nightmares_Character_C|GetIsADS _asnightmares_character) 0.25 (select (and (> (.X (Math|Vector2D|BreakVector2D _returnvalue_3)) 0.0) (Variables|Default|GetIsSprinting)) 1.0 0.5))))) false))

(event Input|EnhancedActionEvents|EnhancedInputActionIA_OniKami_Look
  (params (ActionValue :type Vector%202D%20Structure) (ElapsedSeconds :type Float%20%28double-precision%29) (TriggeredSeconds :type Float%20%28double-precision%29) (InputAction :type Input%20Action%20Object%20Reference :default "/Game/Nightmares/Inputs/IA_OniKami_Look.IA_OniKami_Look"))
  (bind _playercameramanager (Variables|Default|GetPlayerCameraManager))
  (bind _controllersensitivity (Variables|Default|GetControllerSensitivity))
  (bind _returnvalue (Camera|GetFOVAngle _playercameramanager))
  (bind _returnvalue_2 (/ _returnvalue 9e+01))
  (bind _returnvalue_3 (* _controllersensitivity _returnvalue_2))
  (bind _returnvalue_4 (* ActionValue _returnvalue_3))
  (bind (_x _y) (Math|Vector2D|BreakVector2D _returnvalue_4))
  (Class|PlayerController|AddYawInput _x)
  (Class|PlayerController|AddPitchInput _y))

(event EventPossess
  (params (PossessedPawn :type Pawn%20Object%20Reference))
  (Class|PlayerController|ClientSetHUD "/Game/Nightmares/Blueprints/HUDs/Game.Game_C"))

(event Input|KeyboardEvents|Escape
  (params (Key :type Key%20Structure :default "None"))
  (:Pressed
    (bind _asnightmares_hud (Utilities|Casting|CastToNightmares_HUD (HUD|GetHUD)))
    (Default|Open _asnightmares_hud "/Game/Nightmares/UserWidgets/Game/WBP_StfGame_Pause.WBP_StfGame_Pause_C" "NewEnumerator0")))

(event Input|KeyboardEvents|Tab
  (params (Key :type Key%20Structure :default "None"))
  (:Pressed
    (bind _asnightmares_hud (Utilities|Casting|CastToNightmares_HUD (HUD|GetHUD)))
    (Default|Open _asnightmares_hud "/Game/Nightmares/UserWidgets/Game/WBP_Nightmares_PlayerInventory.WBP_Nightmares_PlayerInventory_C" "NewEnumerator0")))

(event Input|KeyboardEvents|LeftShift
  (params (Key :type Key%20Structure :default "None"))
  (:Pressed
    (Variables|Default|SetIsSprinting true))
  (:Released
    (Variables|Default|SetIsSprinting false)))

(event Input|KeyboardEvents|P
  (params (Key :type Key%20Structure :default "None"))
  (:Pressed
    (bind _asnightmares_hud (Utilities|Casting|CastToNightmares_HUD (HUD|GetHUD)))
    (Default|Open _asnightmares_hud "/Game/Nightmares/UserWidgets/Game/WBP_StfGame_Pause.WBP_StfGame_Pause_C" "NewEnumerator0")))

(fn ConstructionScript)

(fn ReceiveBeginPlay
  (bind _returnvalue (PlayerController|LocalPlayerSubsystems|GetEnhancedInputLocalPlayerSubsystem))
  (Utilities|IsValid _returnvalue
    (:Is%20Valid
      (Input|AddMappingContext _returnvalue "/Game/Nightmares/Inputs/IMC_OniKami.IMC_OniKami" 0 "(bIgnoreAllPressedKeysUntilRelease=True,bForceImmediately=False,bNotifyUserSettings=False)"))))

(fn Spawn
  (Class|GameModeBase|RestartPlayer (Game|GetGameMode) self))

(fn ReceiveTick
  (params (DeltaSeconds :type Float%20%28single-precision%29))
  (|CallParentFunction DeltaSeconds)
  (if (Networking|IsServer)
    (if (Variables|Default|GetIsDead)
      _)))

(fn Die
  (Class|PlayerController|ClientSetHUD "/Game/Nightmares/Blueprints/HUDs/Dead.Dead_C")
  (Variables|Default|SetIsDead true))