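; Pickup generator actor that, on the server at BeginPlay, picks a random class from its item property list and constructs a property object from it.
; Spawning a pickup with an inventory, interaction component and random-UUID item is present but disconnected, as are the inventory-removal binding and actor destruction.
; The removal handler compares the item's UUID to the first inventory entry but takes no action, so no pickup is generated.
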(event Custom|CustomEvent
  (params (Item :type Nightmares%20Item%20Structure))
  (if (Utilities|Enum|Equal(Enum) (.UUID (Utilities|Struct|BreakNightmares_Item Item)) (.UUID (Utilities|Struct|BreakNightmares_Item (Utilities|Array|Get(acopy) (Variables|/Game/InventoryV2/V2Inventory.V2Inventory_C|GetItems (Actor|GetComponentbyClass "/Game/InventoryV2/V2Inventory.V2Inventory_C"))))))
    _))

(event EventBeginPlay
  (if (Networking|IsServer)
    (Variables|Default|SetPropertyClass (.OutItem (Utilities|Array|Random (Variables|Default|GetItemsProperty))))
    (bind _returnvalue (Game|ConstructObjectfromClass (Variables|Default|GetPropertyClass)))
    (Variables|Default|SetProperty _returnvalue)))

(fn ConstructionScript)