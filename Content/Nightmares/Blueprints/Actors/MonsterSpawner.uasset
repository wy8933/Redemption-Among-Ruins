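; MonsterSpawner is a server-side spawner actor that keeps a small population of Nightmares_Wanderer monsters around itself while players are nearby.
; On BeginPlay the server starts a looping timer that checks whether any player's pawn is within range.
; If so, it counts BP_AIC_Zombie controllers whose Spawner references it and spawns wanderers at random horizontal offsets up to the cap.
; Each new monster gets its default AI controller, tagged with this spawner for later counts.
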(event Custom|CustomEvent
  (Variables|Default|SetHasPlayersNeared false)
  (bind _outactors (Actor|GetAllActorsOfClass "/Script/Engine.PlayerController"))
  (for _array_element _outactors
    (if (< (Transformation|GetDistanceTo (Pawn|GetControlledPawn _array_element) self) 1e+04)
      (Variables|Default|SetHasPlayersNeared true)))
  (if (Variables|Default|GetHasPlayersNeared)
    (Variables|Default|SetKids 0)
    (bind _outactors_2 (Actor|GetAllActorsOfClass "/Game/Nightmares/AI/Zombie/BP_AIC_Zombie.BP_AIC_Zombie_C"))
    (for _array_element_2 _outactors_2
      (if (== (Variables|/Game/Nightmares/AI/Zombie/BP_AIC_Zombie.BP_AIC_Zombie_C|GetSpawner _array_element_2) self)
        (Math|Integer|IncrementInt (Variables|Default|GetKids))))
    (if (> (- 5 (Variables|Default|GetKids)) 0)
      (for _index (range 1 (- 5 (Variables|Default|GetKids)))
        (bind _returnvalue (Game|SpawnActorfromClass "/Game/Nightmares/Blueprints/Characters/Nightmares_Wanderer.Nightmares_Wanderer_C" (Math|Transform|MakeTransform (+ (Transformation|GetActorLocation) (Math|Vector|MakeVector (Math|Random|RandomFloatinRange -3e+03 3e+03) (Math|Random|RandomFloatinRange -3e+03 3e+03) 0.0)) (Transformation|GetActorRotation) "1.000000,1.000000,1.000000") "Undefined" "MultiplyWithRoot" self 0))
        (Pawn|SpawnDefaultController _returnvalue)
        (bind _asbp_aic_zombie (Utilities|Casting|CastToBP_AIC_Zombie (Pawn|GetController _returnvalue)))
        (Variables|/Game/Nightmares/AI/Zombie/BP_AIC_Zombie.BP_AIC_Zombie_C|SetSpawner _asbp_aic_zombie self)))))

(event EventBeginPlay
  (if (Networking|IsServer)
    (Utilities|Time|SetTimerbyEvent (delegate Custom|CustomEvent) 2.0 true)))

(fn ConstructionScript)

(fn ReceiveTick
  (params (DeltaSeconds :type Float%20%28single-precision%29)))