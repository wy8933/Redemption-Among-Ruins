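; Game instance for Nightmares that handles graphics and audio settings and creates the quest monitors.
; Graphics options go straight to GameUserSettings, while volume, language and subtitle options persist in a Save_Settings slot, lazily loaded or created and then cached.
; Init re-sends saved audio settings through SaveAudioSettingMessage after a short delay, then builds a map of monitor objects from DT_Quests, keyed by row name.
; The sound mix volume overrides are disconnected and never run.
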(event EventApplyGraphicsSetting
  (params (anti%20aliasing :type Integer) (shadow%20qulity :type Integer) (texture%20quality :type Integer) (foliage%20quality :type Integer) (process%20quality :type Integer) (view%20distance :type Integer) (v%20sync :type Boolean))
  ;[1 1 1] Apply graphics settings to the game
  (bind _returnvalue (Settings|GetGameUserSettings))
  (Class|GameUserSettings|SetAntiAliasingQuality _returnvalue anti%20aliasing)
  (Class|GameUserSettings|SetShadowQuality _returnvalue shadow%20qulity)
  (Class|GameUserSettings|SetTextureQuality _returnvalue texture%20quality)
  (Class|GameUserSettings|SetFoliageQuality _returnvalue foliage%20quality)
  (Class|GameUserSettings|SetPostProcessingQuality _returnvalue process%20quality)
  (Class|GameUserSettings|SetViewDistanceQuality _returnvalue view%20distance)
  (Class|GameUserSettings|SetVSyncEnabled _returnvalue v%20sync)
  (Class|GameUserSettings|ApplySettings _returnvalue true))

(event EventSaveAudioSetting
  (params (masterVolumn :type Float%20%28double-precision%29) (musicVolume :type Float%20%28double-precision%29) (sfxVolumn :type Float%20%28double-precision%29) (voiceVolumn :type Float%20%28double-precision%29) (audioLanguage :type Integer) (subtitleLanguage :type Integer) (subtitleEnabled :type Integer))
  (bind _save_settings (Variables|Default|GetSave%20Settings))
  (Utilities|LoadSettings
    (:OutputPin
      (Variables|/Game/Nightmares/SaveGames/Save_Settings.Save_Settings_C|SetmasterVolume _save_settings masterVolumn)
      (Variables|/Game/Nightmares/SaveGames/Save_Settings.Save_Settings_C|SetmusicVolume _save_settings musicVolume)
      (Variables|/Game/Nightmares/SaveGames/Save_Settings.Save_Settings_C|SetsfxVolume _save_settings sfxVolumn)
      (Variables|/Game/Nightmares/SaveGames/Save_Settings.Save_Settings_C|SetvoiceVolume _save_settings voiceVolumn)
      (Variables|/Game/Nightmares/SaveGames/Save_Settings.Save_Settings_C|SetaudioLanguage _save_settings audioLanguage)
      (Variables|/Game/Nightmares/SaveGames/Save_Settings.Save_Settings_C|SetsubtitleLanguage _save_settings subtitleLanguage)
      (Variables|/Game/Nightmares/SaveGames/Save_Settings.Save_Settings_C|SetsubtitleEnabled _save_settings subtitleEnabled)
      (SaveGame|SaveGametoSlot (Variables|Default|GetSave%20Settings) (Variables|Default|GetSlotName_Setting)))))

(event EventInit
  (Utilities|FlowControl|Sequence
    (:then_0
      (|ReloadAudioSettings))
    (:then_1
      (bind _outrownames (DataTable|GetDataTableRowNames "/Game/Nightmares/Quest/DT_Quests.DT_Quests"))
      (for _array_element _outrownames
        (bind _returnvalue (Utilities|GetDataTableRow "/Game/Nightmares/Quest/DT_Quests.DT_Quests" _array_element)
          (:then
            (bind _returnvalue_2 (Game|ConstructObjectfromClass (.QuestMonitorClass (Utilities|Struct|BreakF_Quest _returnvalue))))
            (Utilities|Map|Add (Variables|Default|GetQuestMonitors) _array_element _returnvalue_2)))))))

(fn GetSettings
  (bind _save_settings (Utilities|LoadSettings)
    (:OutputPin
      (return _save_settings))))