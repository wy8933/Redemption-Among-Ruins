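; Lobby game mode that starts the match once every player is ready.
; Each tick until the game starts, it checks all BP_PS_Lobby player states, requiring at least one and all flagged Ready.
; When that passes, it latches GameStarted, waits briefly, then runs a ServerTravel console command to the Nightmares_CentralPlaza map.
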(event EventTick
  (params (DeltaSeconds :type Float%20%28single-precision%29))
  (|CallParentFunction DeltaSeconds)
  (if (not (Variables|Default|GetGameStarted))
    (if (CallFunction|CheckShouldStartGame)
      (Variables|Default|SetGameStarted true)
      (Utilities|FlowControl|Delay 2.0)
      (Development|ExecuteConsoleCommand "ServerTravel /Game/Users/WJ/Nightmares_CentralPlaza" 0))))

(fn ConstructionScript)

(fn CheckShouldStartGame
  (bind _outactors (Actor|GetAllActorsOfClass "/Game/Nightmares/Blueprints/PlayerStates/BP_PS_Lobby.BP_PS_Lobby_C"))
  (if (> (Utilities|Array|Length _outactors) 0)
    (for _array_element _outactors
      (if (not (Variables|/Game/Nightmares/Blueprints/PlayerStates/BP_PS_Lobby.BP_PS_Lobby_C|GetReady _array_element))
        (return false)))
    (return true)
    (else
      (return false))))