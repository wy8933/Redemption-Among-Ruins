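; Player character for Nightmares with crouch, jump, lean, aim, FPS camera toggle and interaction.
; Tick sphere-traces from the camera for interactable actors, forward-traces to drive HandClip, and counts down ability cooldown on the server.
; Server-named events route interaction, inventory pickup, teammate respawn and damage; death notifies the controller and ragdolls through NetAll events.
; Reload, drop, firing and held-item logic are mostly empty or disconnected.
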(event Custom|ServerSpawnTeammates
  (params (Point :type Revive%20Point%20Object%20Reference))
  (bind _outactors (Actor|GetAllActorsOfClass "/Game/Nightmares/Blueprints/PlayerControllers/BP_PC_Nightmares.BP_PC_Nightmares_C"))
  (for _array_element _outactors
    (Utilities|IsValid (Pawn|GetControlledPawn _array_element)
      (:Is%20Not%20Valid
        (Class|GameModeBase|RestartPlayeratTransform (Game|GetGameMode) _array_element (Transformation|GetActorTransform Point))))))

(event Custom|NetAllSpawnHitEffect
  (params (Location :type Vector))
  (Niagara|SpawnSystematLocation "/Game/Nightmares/Effects/Nightmares_BloodEffect.Nightmares_BloodEffect" Location (Math|Rotator|FindLookatRotation (Transformation|GetActorLocation) Location)))

(event Custom|ServerStartHold
  (params (Item :type Nightmares%20Global%20Item%20ID%20Structure))
  (CallFunction|StartHold))

(event Custom|NetAllPlayAnimMontage
  (params (AnimMontage :type Anim%20Montage%20Object%20Reference))
  (for _array_element (Utilities|Array|MakeArray (Variables|Character|GetMesh) 0)
    (Animation|Montage|PlayMontage _array_element AnimMontage)))

(event Custom|NetAllSimulate
  (Collision|SetCollisionEnabled (Variables|Collision|GetCapsuleComponent) "NoCollision")
  (Physics|SetSimulatePhysics (Variables|Character|GetMesh) true))

(event Custom|NetAllPlayDieSound)

(event Custom|NetAllSetMaxWalkSpeed
  (params (MaxWalkSpeed :type Float%20%28single-precision%29))
  (Variables|/Script/Engine.CharacterMovementComponent|SetMaxWalkSpeed (Variables|Character|GetCharacterMovement) MaxWalkSpeed))

(event Custom|ServerInteract
  (params (Actor :type Actor%20Object%20Reference))
  (Class|Interaction|Interact(Message) Actor self))

(event Custom|ServerDrop
  (params (Item :type Nightmares%20Global%20Item%20ID%20Structure))
  (CallFunction|Drop))

(event Custom|ServerReload)

(event Custom|ServerEndProgress
  (params (Target :type Object%20Object%20Reference))
  (Class|Interaction|EndProgress(Message) Target))

(event Custom|ServerTakeDamage
  (params (Target :type Self%20Object%20Reference) (HealthOff :type Float%20%28double-precision%29) (Location :type Vector) (From :type Player%20State%20Object%20Reference))
  (CallFunction|TakeDamage Target HealthOff Location From))

(event Custom|ServerPickUp
  (params (FromInventory :type V2%20Inventory%20Object%20Reference) (FromUUID :type String))
  (CallFunction|PickUp FromInventory FromUUID))

(event Input|MouseEvents|RightMouseButton
  (params (Key :type Key%20Structure :default "None"))
  (:Pressed
    (Variables|Default|SetIsADS true))
  (:Released
    (Variables|Default|SetIsADS false)))

(event Input|KeyboardEvents|E
  (params (Key :type Key%20Structure :default "None"))
  (:Pressed
    (Math|Float|IncrementFloat (Variables|Default|GetPeek)))
  (:Released
    (Math|Float|DecrementFloat (Variables|Default|GetPeek))))

(event Input|KeyboardEvents|Q
  (params (Key :type Key%20Structure :default "None"))
  (:Pressed
    (Math|Float|DecrementFloat (Variables|Default|GetPeek)))
  (:Released
    (Math|Float|IncrementFloat (Variables|Default|GetPeek))))

(event Input|KeyboardEvents|LeftCtrl
  (params (Key :type Key%20Structure :default "None"))
  (:Pressed
    (if (not (AI|Components|NavMovement|IsFalling (Variables|Character|GetCharacterMovement)))
      (Character|Crouch)))
  (:Released
    (Character|UnCrouch)))

(event Input|KeyboardEvents|F
  (params (Key :type Key%20Structure :default "None"))
  (:Pressed
    (bind _interactingactor (Variables|Default|GetInteractingActor)
      (:then
        (CallFunction|ServerInteract _interactingactor))
      (:else)))
  (:Released
    (bind _interactingactor_2 (Variables|Default|GetInteractingActor)
      (:then
        (CallFunction|ServerEndProgress _interactingactor_2))
      (:else))))

(event Input|KeyboardEvents|R
  (params (Key :type Key%20Structure :default "None"))
  (:Pressed
    (CallFunction|ServerReload)))

(event Input|KeyboardEvents|SpaceBar
  (params (Key :type Key%20Structure :default "None"))
  (:Pressed
    (Character|UnCrouch)
    (Character|Jump))
  (:Released
    (Character|StopJumping)))

(event Input|MouseEvents|LeftMouseButton
  (params (Key :type Key%20Structure :default "None")))

(event Input|KeyboardEvents|V
  (params (Key :type Key%20Structure :default "None"))
  (:Pressed
    (bind _asnightmares_pcm (Utilities|Casting|CastToNightmares_PCM (Game|GetPlayerCameraManager 0)))
    (Variables|/Game/Nightmares/Blueprints/PlayerCameraManager/Nightmares_PCM.Nightmares_PCM_C|SetFPS _asnightmares_pcm (not (Variables|/Game/Nightmares/Blueprints/PlayerCameraManager/Nightmares_PCM.Nightmares_PCM_C|GetFPS _asnightmares_pcm)))))

(fn ConstructionScript)

(fn TakeDamage
  (params (HealthOff :type Float%20%28double-precision%29) (Location :type Vector) (From :type Player%20State%20Object%20Reference))
  (Variables|Default|SetHealth (- (Variables|Default|GetHealth) HealthOff))
  (CallFunction|NetAllSpawnHitEffect Location)
  (if (<= (Variables|Default|GetHealth) 0.0)
    (CallFunction|Die From)))

(fn GetMaxHP
  (Utilities|IsValid (Variables|GetPlayerState)))

(fn SpawnInstance
  (params (InstanceClass :type Actor%20Class%20Reference))
  (bind _self self)
  (bind _returnvalue (Game|SpawnActorfromClass InstanceClass (Math|Transform|MakeTransform "0, 0, 0" "0, 0, 0" "1.000000,1.000000,1.000000") "Undefined" "MultiplyWithRoot" _self _self))
  (return _returnvalue))

(fn Die
  (params (From :type Player%20State%20Object%20Reference))
  (if (not (Variables|Default|GetIsDead))
    (Variables|Default|SetIsDead true)
    (CallFunction|NetAllPlayDieSound)
    (Utilities|FlowControl|Sequence
      (:then_0
        (bind _asbp_pc_nightmares (Utilities|Casting|CastToBP_PC_Nightmares (Pawn|GetController)))
        (Default|Die _asbp_pc_nightmares))
      (:then_1
        (Pawn|Components|CharacterMovement|SetMovementMode (Variables|Character|GetCharacterMovement) "MOVE_None" 0)
        (CallFunction|NetAllSimulate)
        (Actor|SetLifeSpan 1e+01)
        (Class|Pawn|DetachfromControllerPendingDestroy)))))

(fn GetAbility
  (return 0))

(fn ReceiveTick
  (params (DeltaSeconds :type Float%20%28single-precision%29))
  (bind _returnvalue (Transformation|GetActorLocation))
  (bind _returnvalue_2 (Game|GetPlayerCameraManager 0))
  (bind _returnvalue_3 (Camera|GetCameraLocation _returnvalue_2))
  (Utilities|FlowControl|Sequence
    (:then_0
      (if (Pawn|IsLocallyControlled)
        (bind _outhit (Collision|SphereTraceForObjects _returnvalue_3 (+ _returnvalue_3 (* (Math|Vector|GetForwardVector (Camera|GetCameraRotation _returnvalue_2)) 1.5e+02)) 2e+01 (Utilities|Array|MakeArray "ObjectTypeQuery4") false (CallFunction|GetIgnoreItems) "None"))
        (Utilities|IsValid (.HitActor (Collision|BreakHitResult _outhit))
          (:Is%20Valid
            (if (and (Utilities|DoesObjectImplementInterface (.HitActor (Collision|BreakHitResult _outhit)) "/Game/Nightmares/Blueprints/Interfaces/Interaction.Interaction_C") (Utilities|IsValid (Actor|GetComponentbyClass (.HitActor (Collision|BreakHitResult _outhit)) "/Game/Nightmares/Blueprints/ActorComponents/AC_Nightmares_Interaction.AC_Nightmares_Interaction_C")))
              (Variables|Default|SetInteractingActor (.HitActor (Collision|BreakHitResult _outhit)))
              (else
                (Variables|Default|SetInteractingActor 0 :!label _label))))
          (:Is%20Not%20Valid
            (goto _label)))))
    (:then_1
      (if (Networking|IsServer)
        (Variables|Default|SetAbilityCooldown (- (Variables|Default|GetAbilityCooldown) DeltaSeconds))))
    (:then_2
      (bind (_outhit_2 _returnvalue_4) (Collision|LineTraceForObjects _returnvalue (+ _returnvalue (* (Math|Vector|GetForwardVector (Transformation|GetActorRotation)) 1e+02)) (Utilities|Array|MakeArray "ObjectTypeQuery1" "ObjectTypeQuery2") false (Utilities|Array|MakeArray (Variables|Default|GetInteractingActor)) "None"))
      (if _returnvalue_4
        (Variables|Default|SetHandClip (Math|Float|MapRangeClamped (Math|Vector|Distance(Vector) (.Location (Collision|BreakHitResult _outhit_2)) (Transformation|GetActorLocation)) 5e+01 1e+02 1.0 0.0))
        (else
          (Variables|Default|SetHandClip 0.0))))))

(fn ReceiveDestroyed
  (if (Networking|IsServer)
    (Utilities|FlowControl|Sequence)))

(fn PickUp
  (params (FromInventory :type V2%20Inventory%20Object%20Reference) (FromUUID :type String))
  (bind _v2inventory (Variables|Default|GetV2Inventory))
  (Default|Put _v2inventory FromInventory FromUUID _v2inventory (.UUID (Utilities|Struct|BreakNightmares_Item (Utilities|Array|Get(acopy) (Variables|/Game/InventoryV2/V2Inventory.V2Inventory_C|GetItems _v2inventory)))) "Backpack"))

(fn Drop
  (params (Item :type %20Object%20Reference)))

(fn StartHold
  (params (Item :type Nightmares%20Global%20Item%20ID%20Structure))
  (Utilities|FlowControl|Sequence
    (:then_0
      (Variables|Default|GetInstance
        (:then
          (Actor|DestroyActor))
        (:else)))))

(fn DestroyInstance
  (params (Container :type %20Object%20Reference))
  (bind _instance (Variables|Default|GetInstance)
    (:then
      (Actor|DestroyActor _instance))
    (:else)))

(fn GetIgnoreItems
  (Utilities|FlowControl|Sequence
    (:then_1
      (return (LocalVariables|GetItems)))))

(fn GetADSOffset
  (Utilities|FlowControl|Sequence
    (:then_1
      (return "0, 0, 0"))))

(fn GetADSPoint
  (params (Instance :type %20Object%20Reference))
  (for _array_element (Actor|GetAllChildActors true)
    (for _array_element_2 (Actor|GetComponentsbyTag _array_element "/Script/Engine.SceneComponent" "ADS")
      (return _array_element_2)))
  (for _array_element_3 (Actor|GetComponentsbyTag "/Script/Engine.SceneComponent" "ADS")
    (return _array_element_3))
  (return 0))

(fn ReceiveBeginPlay
  (if (Networking|IsServer)
    (Variables|/Game/InventoryV2/V2Inventory.V2Inventory_C|SetItems (Variables|Default|GetV2Inventory) (Utilities|Array|MakeArray (Utilities|Struct|MakeNightmares_Item (Utilities|String|ToString(Integer) (Math|Random|RandomInteger 2147483647)) 0)))))