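; Nightmares HUD that manages a stack of menu widgets and the matching player input mode.
; Open creates a widget, adds it to the viewport, pushes it with its input mode and centers the mouse; Back removes and pops the top entry.
; Both then call Apply, which sets cursor visibility and UI, game or combined input from the top entry.
; All widgets are removed on end play.
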(fn ConstructionScript)

(fn Apply
  (bind _returnvalue (Game|GetPlayerController 0))
  (bind _menus (Variables|Default|GetMenus))
  (bind _returnvalue_2 (Utilities|Array|LastIndex _menus))
  (bind _output (Utilities|Array|Get(acopy) _menus _returnvalue_2))
  (bind (_uw _inputmode) (Utilities|Struct|BreakF_StfGame_MenuState _output))
  (Variables|/Script/Engine.PlayerController|SetbShowMouseCursor (Game|Player|GetOwningPlayerController) (Utilities|Enum|NotEqual(Enum) _inputmode "NewEnumerator1"))
  (switch Utilities|FlowControl|Switch|SwitchonE_StfGame_InputMode _inputmode
    (:NewEnumerator0
      (Input|SetInputModeUIOnly _returnvalue _uw "DoNotLock" true))
    (:NewEnumerator1
      (Input|SetInputModeGameOnly _returnvalue false))
    (:NewEnumerator2
      (Input|SetInputModeGameandUI _returnvalue _uw "DoNotLock" true false))))

(fn Open
  (params (UWClass :type User%20Widget%20Class%20Reference) (InputMode :type E_StfGame_InputMode%20Enum :default "NewEnumerator0"))
  (bind _returnvalue (Viewport|GetViewportSize))
  (bind (_x _y) (Math|Vector2D|BreakVector2D _returnvalue))
  (bind _returnvalue_2 (UserInterface|CreateWidget UWClass))
  (bind _output_get (LocalVariables|SetMenu _returnvalue_2))
  (UserInterface|Viewport|AddtoViewport _output_get 0)
  (Utilities|Array|Add (Variables|Default|GetMenus) (Utilities|Struct|MakeF_StfGame_MenuState (LocalVariables|GetMenu) InputMode))
  (CallFunction|Apply)
  (Class|PlayerController|SetMouseLocation (Game|Player|GetOwningPlayerController) (Math|Float|Truncate (/ _x 2.0)) (Math|Float|Truncate (/ _y 2.0))))

(fn Back
  (bind _menus (Variables|Default|GetMenus))
  (bind _menus_2 (Variables|Default|GetMenus))
  (Widget|RemovefromParent (.UW (Utilities|Struct|BreakF_StfGame_MenuState (Utilities|Array|Get(acopy) _menus_2 (Utilities|Array|LastIndex _menus_2)))))
  (Utilities|Array|RemoveIndex _menus (Utilities|Array|LastIndex _menus))
  (CallFunction|Apply))

(fn ReceiveEndPlay
  (params (EndPlayReason :type EEndPlayReason%20Enum :default "Destroyed"))
  (Viewport|RemoveAllWidgets))