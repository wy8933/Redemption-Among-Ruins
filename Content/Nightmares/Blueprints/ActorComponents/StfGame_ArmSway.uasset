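; Actor component that produces a combined arm sway offset for a Character from a set of pluggable calculation objects.
; On BeginPlay it constructs one object per entry in its class list, passing in the owning Character.
; Output runs each calculation with the world delta time, adding location offsets and combining rotation offsets into a single returned pair.
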(event EventBeginPlay
  (for _array_element (Variables|Default|GetCalculationClass)
    (bind _ascharacter (Utilities|Casting|CastToCharacter (Components|GetOwner)))
    (bind _returnvalue (Game|ConstructObjectfromClass _array_element _ascharacter))
    (Utilities|Array|Add (Variables|Default|GetCalculations) _returnvalue)))

(fn Output
  (for _array_element (Variables|Default|GetCalculations)
    (bind (_offsetlocation _offsetrotation) (Default|Output _array_element (Utilities|Time|GetWorldDeltaSeconds)))
    (LocalVariables|SetLocation (+ (LocalVariables|GetLocation) _offsetlocation))
    (LocalVariables|SetRotation (Math|Rotator|CombineRotators (LocalVariables|GetRotation) _offsetrotation)))
  (return (LocalVariables|GetLocation) (LocalVariables|GetRotation)))