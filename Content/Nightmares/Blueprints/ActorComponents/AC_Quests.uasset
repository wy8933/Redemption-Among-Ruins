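; AC_Quests is an actor component that tracks completed quests and plays a sound when a quest passes.
; On server BeginPlay, it reads the QuestMonitors map from Nightmares_GI and adds keys of already-passed monitors to SavedQuests.
; It then binds every monitor's OnPass event to a handler that plays the quest-completion sound in 2D.
; SavedQuests is not updated by that handler.
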(event Custom|CustomEvent
  (Audio|PlaySound2D "/Game/StfContent/Audio/quest_c.quest_c" 1.0 1.0 0.0 0 0))

(event EventBeginPlay
  (if (Networking|IsServer)
    (bind _asnightmares_gi (Utilities|Casting|CastToNightmares_GI (Game|GetGameInstance)))
    (Utilities|FlowControl|Sequence
      (:then_0
        (bind _keys (Utilities|Map|Keys (Variables|/Game/Nightmares/Blueprints/GameInstances/Nightmares_GI.Nightmares_GI_C|GetQuestMonitors _asnightmares_gi)))
        (for (_array_element _array_index) _keys
          (bind _values (Utilities|Map|Values (Variables|/Game/Nightmares/Blueprints/GameInstances/Nightmares_GI.Nightmares_GI_C|GetQuestMonitors _asnightmares_gi)))
          (if (Variables|/Game/Nightmares/Quest/BP_QuestMonitor.BP_QuestMonitor_C|GetPassed (Utilities|Array|Get(acopy) _values _array_index))
            (Utilities|Array|Add (Variables|Default|GetSavedQuests) _array_element))))
      (:then_1
        (bind _values_2 (Utilities|Map|Values (Variables|/Game/Nightmares/Blueprints/GameInstances/Nightmares_GI.Nightmares_GI_C|GetQuestMonitors _asnightmares_gi)))
        (for _array_element_2 _values_2
          (EventDispatchers|BindEventtoOnPass _array_element_2 (delegate Custom|CustomEvent)))))))