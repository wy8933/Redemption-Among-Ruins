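; Actor component for a Nightmare instance that ties its owning actor's lifetime to an inventory item.
; On BeginPlay, the server binds to the remove event of the inventory referenced by its Item.
; When an item is removed, it compares UUIDs and destroys the owning actor if the removed item is the tracked one.
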(event Custom|CustomEvent_0
  (params (Item :type Nightmares%20Item%20Structure))
  (if (Utilities|Enum|Equal(Enum) (.UUID (Utilities|Struct|BreakNightmares_Item Item)) (.UUID (Utilities|Struct|BreakNightmares_GlobalItemID (Variables|Default|GetItem))))
    (Actor|DestroyActor (Components|GetOwner))))

(event EventBeginPlay
  (if (Networking|IsServer)
    (EventDispatchers|BindEventtoOnRemove (.Inventory (Utilities|Struct|BreakNightmares_GlobalItemID (Variables|Default|GetItem))) (delegate Custom|CustomEvent_0))))