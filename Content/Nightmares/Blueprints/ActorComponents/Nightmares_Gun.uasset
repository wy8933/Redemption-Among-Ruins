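; Gun actor component for a weapon actor, handling fire cooldown, bullet spawning, recoil and procedural sway.
; Tick drives local fire attempts and blends smoothed recoil with velocity-based curve sway and control-rotation lag into FinalSway.
; ServerShoot relays through NetAllShoot so non-locally-controlled copies spawn their own bullets.
; Ammo, reload, recoil amount and attachment functions are stubs, and TryShoot's firing calls are disconnected.
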(event Custom|ServerShoot
  (params (Location :type Vector) (Rotation :type Rotator))
  (CallFunction|NetAllShoot Location Rotation))

(event Custom|NetAllShoot
  (params (Location :type Vector) (Rotation :type Rotator))
  (if (not (Pawn|IsLocallyControlled (Variables|/Script/Engine.Actor|GetInstigator (Components|GetOwner))))
    (CallFunction|Shoot Location Rotation)))

(fn ReceiveTick
  (params (DeltaSeconds :type Float%20%28single-precision%29))
  (Utilities|FlowControl|Sequence
    (:then_0
      (if (Pawn|IsLocallyControlled (Variables|/Script/Engine.Actor|GetInstigator (Components|GetOwner)))
        (Variables|Default|SetCurCD (- (Variables|Default|GetCurCD) DeltaSeconds))
        (if (Variables|Default|GetIsFiring)
          (CallFunction|TryShoot))))
    (:then_1
      (Variables|Default|SetSmoothRecoils (Class|KismetMathLibrary|Vector2DInterpto (Variables|Default|GetSmoothRecoils) (Variables|Default|GetRecoils) DeltaSeconds (Math|Float|MakeLiteralFloat 1e+01)))
      (Variables|Default|SetRecoils (Class|KismetMathLibrary|Vector2DInterpto :Current (Variables|Default|GetRecoils) :DeltaTime DeltaSeconds :InterpSpeed (Math|Float|MakeLiteralFloat 15.0)))
      (Variables|Default|SetFinalSway (Math|Rotator|CombineRotators (Math|Rotator|MakeRotator 0.0 (.Y (Math|Vector2D|BreakVector2D (Variables|Default|GetSmoothRecoils))) (.X (Math|Vector2D|BreakVector2D (Variables|Default|GetSmoothRecoils)))) (Math|Rotator|CombineRotators (Variables|Default|GetMovementSway) (Variables|Default|GetLookSway)))))
    (:then_2
      (CallFunction|UpdateMovementSway)
      (CallFunction|UpdateLookSway))))

(fn Shoot
  (params (Location :type Vector) (Rotation :type Rotator))
  (bind _returnvalue (Components|GetOwner))
  (Game|SpawnActorfromClass "/Game/Nightmares/Blueprints/Bullets/Bullet.Bullet_C" (Math|Transform|MakeTransform Location Rotation "1.000000,1.000000,1.000000") "Undefined" "MultiplyWithRoot" _returnvalue 0 self (Variables|/Script/Engine.Actor|GetInstigator _returnvalue) 0))

(fn GetMuzzlePoint
  (return (Utilities|Array|Get(acopy) (Actor|GetComponentsbyTag (Components|GetOwner) "/Script/Engine.SceneComponent" "FirePoint"))))

(fn GetADSPoint
  (return (Utilities|Array|Get(acopy) (Actor|GetComponentsbyTag (Components|GetOwner) "/Script/Engine.ArrowComponent" "ADS"))))

(fn GetCurrentAmmo
  (return 0))

(fn Reload)

(fn TakeBullet)

(fn UpdateMovementSway
  (bind _returnvalue (Components|GetOwner))
  (bind _returnvalue_2 (Components|GetOwner _returnvalue))
  (Variables|Default|SetSmoothCharacterVec (Math|Interpolation|VInterpTo (Variables|Default|GetSmoothCharacterVec) (Math|Vector|UnrotateVector (Transformation|GetVelocity _returnvalue_2) (Transformation|GetActorRotation _returnvalue_2)) (Utilities|Time|GetWorldDeltaSeconds) 5.0))
  (bind _ascharacter (Utilities|Casting|CastToCharacter (Variables|/Script/Engine.Actor|GetInstigator (Components|GetOwner))))
  (switch Utilities|FlowControl|Switch|SwitchonEMovementMode (Variables|/Script/Engine.CharacterMovementComponent|GetMovementMode (Variables|/Script/Engine.Character|GetCharacterMovement _ascharacter))
    (:MOVE_None
      _)
    (:MOVE_Walking
      _)
    (:MOVE_NavWalking
      _))
  (Variables|Default|SetMovementSwayTime (+ (Variables|Default|GetMovementSwayTime) (* (Utilities|Time|GetWorldDeltaSeconds) (Math|Float|MapRangeClamped (Math|Vector|VectorLength (Math|Vector|MakeVector (.X (Math|Vector|BreakVector (Variables|Default|GetSmoothCharacterVec))) (.Y (Math|Vector|BreakVector (Variables|Default|GetSmoothCharacterVec))) 0.0)) 0.0 4.5e+02 0.0 3.0))))
  (Variables|Default|SetMovementSway (Math|Rotator|MakeRotator (Math|Float|MapRangeClamped (.Y (Math|Vector|BreakVector (Variables|Default|GetSmoothCharacterVec))) -6e+02 6e+02 -4.0 4.0) (.Z (Math|Vector|BreakVector (* (Math|Curves|GetVectorValue (LocalVariables|GetMovementSwayCurve) (Variables|Default|GetMovementSwayTime)) (Math|Float|MapRangeClamped (Math|Vector|VectorLength (Math|Vector|MakeVector (.X (Math|Vector|BreakVector (Variables|Default|GetSmoothCharacterVec))) (.Y (Math|Vector|BreakVector (Variables|Default|GetSmoothCharacterVec))) 0.0)) 0.0 6e+02 0.0 6.0)))) (.Y (Math|Vector|BreakVector (* (Math|Curves|GetVectorValue (LocalVariables|GetMovementSwayCurve) (Variables|Default|GetMovementSwayTime)) (Math|Float|MapRangeClamped (Math|Vector|VectorLength (Math|Vector|MakeVector (.X (Math|Vector|BreakVector (Variables|Default|GetSmoothCharacterVec))) (.Y (Math|Vector|BreakVector (Variables|Default|GetSmoothCharacterVec))) 0.0)) 0.0 6e+02 0.0 6.0)))))))

(fn UpdateLookSway
  (bind _returnvalue (Components|GetOwner))
  (bind _instigator (Variables|/Script/Engine.Actor|GetInstigator _returnvalue))
  (bind _returnvalue_2 (Pawn|GetControlRotation _instigator :!class /Script/Engine.Pawn))
  (Variables|Default|SetLookSway (Math|Interpolation|RInterpTo (Variables|Default|GetLookSway) (* (Math|Rotator|Delta(Rotator) _returnvalue_2 (Variables|Default|GetLastUpdatedControlRotation)) -1.0) (Utilities|Time|GetWorldDeltaSeconds) 7.5))
  (Variables|Default|SetLastUpdatedControlRotation _returnvalue_2))

(fn TryShoot
  (if (Math|Boolean|ANDBoolean (<= (Variables|Default|GetCurCD) 0.0) (> (CallFunction|GetCurrentAmmo) 0) (not (Utilities|IsValid (Animation|GetCurrentMontage (.AsCharacter (Utilities|Casting|CastToCharacter (Variables|/Script/Engine.Actor|GetInstigator (Components|GetOwner)))) :!class /Script/Engine.Character))))
    _))

(fn PushRecoil
  (bind _recoil (CallFunction|GetRecoil))
  (bind _returnvalue (/ _recoil 2.0))
  (Variables|Default|SetRecoils (+ (Variables|Default|GetRecoils) (Math|Vector2D|MakeVector2D (Math|Random|RandomFloatinRange (* _returnvalue -1.0) _returnvalue) (Math|Random|RandomFloatinRange _recoil (* _recoil 2.0))))))

(fn GetRecoil)

(fn GetAttachments
  (params (Item :type %20Object%20Reference)))