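; Slug is a bullet Actor that damages Nightmares_Character targets on impact and then destroys itself.
; On BeginPlay it gives its static mesh a dynamic material with a random color.
; ReceiveHit spawns a temporary bullet-hole decal aligned to the surface normal and, only on the server, passes GetDamage to the hit character's TakeDamage.
; GetDamage returns zero here, so this class deals no damage by itself.
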(event EventBeginPlay
  (bind _returnvalue (Rendering|Material|CreateDynamicMaterialInstance (Variables|Default|GetStaticMesh) 0 0 "None" :!class /Script/Engine.PrimitiveComponent))
  (Rendering|Material|SetVectorParameterValue _returnvalue "Color" (Math|Color|MakeColor (Math|Random|RandomFloatinRange 0.0 1.0) (Math|Random|RandomFloatinRange 0.0 1.0) (Math|Random|RandomFloatinRange 0.0 1.0)) :!class /Script/Engine.MaterialInstanceDynamic))

(fn ConstructionScript)

(fn ReceiveHit
  (params (MyComp :type Primitive%20Component%20Object%20Reference) (Other :type Actor%20Object%20Reference) (OtherComp :type Primitive%20Component%20Object%20Reference) (bSelfMoved :type Boolean) (HitLocation :type Vector :default "0, 0, 0") (HitNormal :type Vector :default "0, 0, 0") (NormalImpulse :type Vector :default "0, 0, 0") (Hit :type Hit%20Result%20Structure%20%28by%20ref%29))
  (Utilities|FlowControl|Sequence
    (:then_0
      (bind _returnvalue (Rendering|Decal|SpawnDecalatLocation "/Game/Nightmares/Textures/M_BulletHole.M_BulletHole" (Math|Conversions|ToVector(Float) 5.0) HitLocation (Math|Conversions|RotationFromXVector HitNormal) 1e+01))
      (Utilities|IsValid _returnvalue
        (:Is%20Valid
          (Rendering|Components|Decal|SetFadeScreenSize _returnvalue 0.0))))
    (:then_1
      (if (Networking|IsServer)
        (bind _asnightmares_character (Utilities|Casting|CastToNightmares_Character Other))
        (Default|TakeDamage _asnightmares_character (CallFunction|GetDamage) HitLocation)))
    (:then_2
      (Actor|DestroyActor))))

(fn GetDamage
  (return 0.0))