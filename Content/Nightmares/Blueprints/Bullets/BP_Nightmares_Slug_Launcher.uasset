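; BP_Nightmares_Slug_Launcher is an explosive launcher projectile that reports a GetDamage value and destroys itself on impact.
; On Hit it spawns a scaled-up explosion emitter at the hit location.
; Only the server then runs a zero-length sphere trace for pawns there and damages the single Nightmares_Character it finds.
; That blast uses its own hardcoded damage, far higher than the GetDamage value.
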(event Collision|EventHit
  (params (MyComp :type Primitive%20Component%20Object%20Reference) (Other :type Actor%20Object%20Reference) (OtherComp :type Primitive%20Component%20Object%20Reference) (bSelfMoved :type Boolean) (HitLocation :type Vector :default "0, 0, 0") (HitNormal :type Vector :default "0, 0, 0") (NormalImpulse :type Vector :default "0, 0, 0") (Hit :type Hit%20Result%20Structure%20%28by%20ref%29))
  (Utilities|FlowControl|Sequence
    (:then_0
      (Effects|SpawnEmitteratLocation "/Game/Explosion/Particles/P_Explosion.P_Explosion" HitLocation "0, 0, 0" "2.500000,2.500000,2.500000")
      (if (Networking|IsServer)
        (bind _outhit (Collision|SphereTraceForObjects HitLocation HitLocation 1e+02 (Utilities|Array|MakeArray "ObjectTypeQuery3") false 0 "None"))
        (bind _asnightmares_character (Utilities|Casting|CastToNightmares_Character (.HitActor (Collision|BreakHitResult _outhit))))
        (Default|TakeDamage _asnightmares_character 1e+02 (.Location (Collision|BreakHitResult _outhit)))))
    (:then_1
      (Actor|DestroyActor))))

(fn ConstructionScript
  (|CallParentFunction))

(fn GetDamage
  (return 2e+01))