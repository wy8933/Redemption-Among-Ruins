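; Player camera manager that sets the view each frame for the Nightmares character in either first or third person.
; An FPS flag switches the location between the mesh's "VB Camera" socket and an over-the-shoulder offset built from control rotation axes, with no collision check.
; Rotation follows the controller's control rotation, while field of view interpolates smoothly toward a target value.
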(fn ConstructionScript)

(fn BlueprintUpdateCamera
  (params (CameraTarget :type Actor%20Object%20Reference))
  (bind _returnvalue (Game|Player|GetOwningPlayerController))
  (bind _returnvalue_2 (Pawn|GetControlRotation _returnvalue :!class /Script/Engine.Controller))
  (bind _asnightmares_character (Utilities|Casting|CastToNightmares_Character CameraTarget))
  (LocalVariables|SetCharacter _asnightmares_character)
  (Variables|Default|SetCurFOV (Math|Interpolation|FInterpTo (Variables|Default|GetCurFOV) (Variables|Default|GetTargetFOV) (Utilities|Time|GetWorldDeltaSeconds) 1e+01))
  (return (select (Variables|Default|GetFPS) (Transformation|GetSocketLocation (Variables|/Script/Engine.Character|GetMesh (LocalVariables|GetCharacter)) "VB Camera") (+ (Transformation|GetActorLocation CameraTarget) (* (Math|Vector|GetForwardVector _returnvalue_2) -2.5e+02) (* (Math|Vector|GetRightVector _returnvalue_2) 5e+01) (* (Math|Vector|GetUpVector _returnvalue_2) 7e+01))) (Pawn|GetControlRotation (Game|Player|GetOwningPlayerController) :!class /Script/Engine.Controller) (Variables|Default|GetCurFOV) true))